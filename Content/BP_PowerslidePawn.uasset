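; Physics-sphere pawn that keeps itself moving and can powerslide by orbiting the nearest actor implementing BP_OrbiterInterface.
; Tick accelerates the sphere while below minimum speed and aligns the spring arm and cone to its velocity.
; Move axes steer by rotating the velocity vector, but are ignored while orbiting.
; Holding Powerslide links the sphere to the orbiter through a spring-driven physics constraint, with a debug line and circle drawn.
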(event `self.ReceiveBeginPlay`
  (`PrimitiveComponent.SetPhysicsLinearVelocity` (`self.Sphere`) (* (`self.GetActorForwardVector`) 10.0) false "None"))

(event `self.ReceiveTick`
  (params (DeltaSeconds :type "Float (single-precision)"))
  (bind _returnvalue (`self.K2_GetActorLocation`))
  (bind _sphere (`self.Sphere`))
  (`|ExecutionSequence`
    (:`then_0`
      (bind _returnvalue_2 (`PrimitiveComponent.GetPhysicsLinearVelocity` _sphere "None"))
      (if (< (`KismetMathLibrary.VSize` _returnvalue_2) (`self.MinimumVelocity`))
        (`PrimitiveComponent.SetPhysicsLinearVelocity` _sphere (+ _returnvalue_2 (* (`KismetMathLibrary.Normal` _returnvalue_2) (* (`self.Acceleration`) DeltaSeconds))) false "None")))
    (:`then_1`
      (bind _returnvalue_3 (`PrimitiveComponent.GetPhysicsLinearVelocity` (`self.Sphere`) "None"))
      (bind _returnvalue_4 (`KismetMathLibrary.MakeRotFromX` (`KismetMathLibrary.Normal` _returnvalue_3)))
      (`SceneComponent.K2_SetWorldRotation` (`self.SpringArm`) _returnvalue_4 false false)
      (`SceneComponent.K2_SetWorldRotation` (`self.Cone`) (`KismetMathLibrary.ComposeRotators` (struct :`Pitch` -90.0) _returnvalue_4) false false))
    (:`then_2`
      (`self.Is Orbiting?`
        (:`True`
          (bind _asactor (cast `Actor` (`KismetSystemLibrary.Conv_InterfaceToObject` (`self.ActiveOrbiter`))))
          (bind _returnvalue_5 (`self.K2_GetActorLocation` _asactor))
          (`KismetSystemLibrary.DrawDebugLine` _returnvalue _returnvalue_5 (struct :`R` 1.0 :`A` 1.0) 0.0 1.0)
          (bind _returnvalue_6 (- _returnvalue _returnvalue_5))
          (`KismetSystemLibrary.DrawDebugCircle` _returnvalue_5 (`KismetMathLibrary.VSize` _returnvalue_6) 128 (struct :`R` 1.0 :`A` 1.0) 0.0 1.0 (`KismetMathLibrary.Normal` _returnvalue_6) (`KismetMathLibrary.Normal` (`self.GetVelocity`)) true))))))

(event `InputAxis|Move X`
  (params (AxisValue :type "Float (single-precision)"))
  (`self.Is Orbiting?`
    (:`False`
      (`self.Handle Rotation` (* AxisValue 2.0) (0.0 0.0 1.0)))))

(event `InputAxis|Move Y`
  (params (AxisValue :type "Float (single-precision)"))
  (`self.Is Orbiting?`
    (:`False`
      (`self.Handle Rotation` (* AxisValue 2.0) (`SceneComponent.GetRightVector` (`self.Cone`))))))

(event `InputAction|Powerslide`
  (params (Key :type "Key Structure" :default "AnyKey"))
  (bind _physicsconstraint (`self.PhysicsConstraint`))
  (bind _physicsconstraint_2 (`self.PhysicsConstraint`))
  (:`Pressed`
    (bind _outactors (`GameplayStatics.GetAllActorsWithInterface` "/Game/BP_OrbiterInterface.BP_OrbiterInterface_C"))
    (bind _closestactor (`self.Find Closest Actor` _outactors))
    (bind _asbp_orbiter_interface (cast `/Game/BP_OrbiterInterface` _closestactor))
    (bind _output_get (set `self.ActiveOrbiter` _asbp_orbiter_interface))
    (`ActorComponent.Activate` (`self.PhysicsConstraint`) false)
    (bind _primitivecomponent (`/Game/BP_OrbiterInterface.GetOrbiterPrimitive` _output_get))
    (`PhysicsConstraintComponent.SetConstrainedComponents` _physicsconstraint _primitivecomponent "None" (`self.Sphere`) "None")
    (`PhysicsConstraintComponent.SetConstraintReferencePosition` _physicsconstraint "Frame1" (0.0 0.0 0.0))
    (`PhysicsConstraintComponent.SetLinearDriveParams` _physicsconstraint 500.0 0.0 0.0)
    (`PhysicsConstraintComponent.SetLinearPositionDrive` _physicsconstraint true true true))
  (:`Released`
    (set `self.ActiveOrbiter` null)
    (`PhysicsConstraintComponent.SetConstrainedComponents` _physicsconstraint_2 null "None" null "None")
    (`PhysicsConstraintComponent.SetLinearPositionDrive` _physicsconstraint_2 false false false)))

(fn `Find Closest Actor`
  (params (Actors :type "Array of Actor Object Reference"))
  (returns (ClosestActor :type "Actor Object Reference"))
  (locals (TempClosestDistance :type "Float (double-precision)") (TempClosestActor :type "Actor Object Reference"))
  (for (_array_element _array_index) Actors
    (if (== _array_index 0)
      (bind _returnvalue (`KismetMathLibrary.VSize` (- (`self.K2_GetActorLocation`) (`self.K2_GetActorLocation` _array_element))))
      (set `local.TempClosestDistance` _returnvalue :!label _label)
      (set `local.TempClosestActor` _array_element)
      (elif (< _returnvalue (`local.TempClosestDistance`))
        (goto _label))))
  (return (`local.TempClosestActor`)))

(fn `GetMovementVector`
  (bind _returnvalue (`PrimitiveComponent.GetPhysicsLinearVelocity` (`self.Sphere`) "None"))
  (if (> (`KismetMathLibrary.VSize` _returnvalue) 0.0)
    _))

(fn `Handle Rotation`
  (params (RotationInput :type "Float (double-precision)") (RotationAxis :type "Vector Structure"))
  (bind _returnvalue (`KismetMathLibrary.RotatorFromAxisAndAngle` RotationAxis RotationInput))
  (bind _sphere (`self.Sphere`))
  (`SceneComponent.K2_AddRelativeRotation` _sphere _returnvalue false false)
  (bind _returnvalue_2 (`PrimitiveComponent.GetPhysicsLinearVelocity` _sphere "None"))
  (`PrimitiveComponent.SetPhysicsLinearVelocity` _sphere (`KismetMathLibrary.GreaterGreater_VectorRotator` _returnvalue_2 _returnvalue) false "None"))

(fn `UserConstructionScript`)